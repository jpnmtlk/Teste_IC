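; BP_Porta_LabInfo is a clickable door with an electronic lock widget, opened by sliding its mesh along a timeline.
; Its trigger box toggles the mouse cursor and click events, and leaving it removes the widget.
; Clicking the door inside that area shows WD_Trava, created on first use and then reused.
; The widget's AbrirPortaED dispatcher drives StatusPorta, which plays the opening timeline when true; the door has no closing logic.
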(event OnClicked(Porta)
  (params (TouchedComponent :type Primitive%20Component%20Object%20Reference) (ButtonPressed :type Key%20Structure :default "AnyKey"))
  (if (Variables|Default|GetPlayerNaArea)
    (if (not (Variables|Default|GetWdAtivo))
      (if (Utilities|IsValid (Variables|Default|GetWD_TravaEletronica))
        (CallFunction|AtivaWD)
        (else
          (bind _returnvalue (UserInterface|CreateWidget "/Game/IC/WD_Trava.WD_Trava_C" (Game|GetPlayerController 0)))
          (bind _output_get (Variables|Default|SetWD_TravaEletronica _returnvalue))
          (EventDispatchers|BindEventtoAbrirPortaED _output_get (delegate Custom|Status%20Porta))
          (CallFunction|AtivaWD))))))

(event OnComponentBeginOverlap(TriggerBox)
  (params (OverlappedComponent :type Primitive%20Component%20Object%20Reference) (OtherActor :type Actor%20Object%20Reference) (OtherComp :type Primitive%20Component%20Object%20Reference) (OtherBodyIndex :type Integer) (bFromSweep :type Boolean) (SweepResult :type Hit%20Result%20Structure%20%28by%20ref%29))
  (bind _returnvalue (Game|GetPlayerController 0))
  (Variables|Default|SetPlayerNaArea true)
  (Variables|/Script/Engine.PlayerController|SetbEnableClickEvents _returnvalue true)
  (Variables|/Script/Engine.PlayerController|SetbShowMouseCursor _returnvalue true))

(event OnComponentEndOverlap(TriggerBox)
  (params (OverlappedComponent :type Primitive%20Component%20Object%20Reference) (OtherActor :type Actor%20Object%20Reference) (OtherComp :type Primitive%20Component%20Object%20Reference) (OtherBodyIndex :type Integer))
  (bind _returnvalue (Game|GetPlayerController 0))
  (Variables|Default|SetPlayerNaArea false)
  (Variables|/Script/Engine.PlayerController|SetbEnableClickEvents _returnvalue false)
  (Variables|/Script/Engine.PlayerController|SetbShowMouseCursor _returnvalue false)
  (CallFunction|DesativaWd))

(event Custom|Status%20Porta
  (params (StatusPorta :type Boolean))
  (if StatusPorta
    (bind _aberturaporta (Timeline|TL%20Porta Play)
      (:Update
        (Transformation|SetRelativeLocation (Variables|Default|GetPorta) _aberturaporta false false)
        (Variables|Default|SetPortaAberta true)))))

(event Custom|Ativa%20WD
  (UserInterface|Viewport|AddtoViewport (Variables|Default|GetWD_TravaEletronica) 0)
  (Variables|Default|SetWdAtivo true))

(event Custom|Desativa%20Wd
  (Widget|RemovefromParent (Variables|Default|GetWD_TravaEletronica))
  (Variables|Default|SetWdAtivo false))

(event EventBeginPlay)

(event Collision|EventActorBeginOverlap
  (params (OtherActor :type Actor%20Object%20Reference)))

(event EventTick
  (params (DeltaSeconds :type Float%20%28single-precision%29)))

(fn ConstructionScript)