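; Light box actor that shows an interaction widget when its trigger box is entered while the lights are off.
; On overlap it lazily creates and caches the WD_CaixaDeLuz widget, adds it to the viewport, turns on the first-person character's mouse cursor and hands the widget a self-reference.
; Leaving the box removes the widget and hides the cursor; both handlers do nothing once LuzesEstaoAcesas is true.
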(event OnComponentBeginOverlap(Box)
  (params (OverlappedComponent :type Primitive%20Component%20Object%20Reference) (OtherActor :type Actor%20Object%20Reference) (OtherComp :type Primitive%20Component%20Object%20Reference) (OtherBodyIndex :type Integer) (bFromSweep :type Boolean) (SweepResult :type Hit%20Result%20Structure%20%28by%20ref%29))
  (if (not (Variables|Default|GetLuzesEstaoAcesas?))
    (if (Utilities|IsValid (Variables|Default|GetWD_CaixaReference))
      _
      (else
        (bind _returnvalue (UserInterface|CreateWidget "/Game/IC/Widgets/WD_CaixaDeLuz.WD_CaixaDeLuz_C"))
        (bind _output_get (Variables|Default|SetWD_CaixaReference _returnvalue))))
    (UserInterface|Viewport|AddtoViewport _output_get 0)
    (Default|VisibilityMouseCursor (.AsFirst%20Person%20Character (Utilities|Casting|CastToFirstPersonCharacter (Game|Player|GetPlayerPawn 0))) true)
    (Variables|/Game/IC/Widgets/WD_CaixaDeLuz.WD_CaixaDeLuz_C|SetCaixaReferences (Variables|Default|GetWD_CaixaReference) self)))

(event OnComponentEndOverlap(Box)
  (params (OverlappedComponent :type Primitive%20Component%20Object%20Reference) (OtherActor :type Actor%20Object%20Reference) (OtherComp :type Primitive%20Component%20Object%20Reference) (OtherBodyIndex :type Integer))
  (if (not (Variables|Default|GetLuzesEstaoAcesas?))
    (Widget|RemovefromParent (Variables|Default|GetWD_CaixaReference))
    (Default|VisibilityMouseCursor (.AsFirst%20Person%20Character (Utilities|Casting|CastToFirstPersonCharacter (Game|Player|GetPlayerPawn 0))) false)))

(event EventBeginPlay)

(event Collision|EventActorBeginOverlap
  (params (OtherActor :type Actor%20Object%20Reference)))

(event EventTick
  (params (DeltaSeconds :type Float%20%28single-precision%29)))

(fn ConstructionScript)