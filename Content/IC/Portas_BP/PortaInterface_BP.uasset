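; PortaInterface_BP is a lockable door that opens on trigger overlap and can be unlocked through the player's inventory.
; If locked, entering the trigger shows the cursor and enables click events, so clicking the door toggles the FirstPersonCharacter's inventory.
; Destranca clears the lock, hides the inventory and plays the yaw timeline that swings the door open.
; Leaving the trigger restores game-only input and reverses the timeline after a short delay.
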(event OnClicked(Porta)
  (params (TouchedComponent :type Primitive%20Component%20Object%20Reference) (ButtonPressed :type Key%20Structure :default "AnyKey"))
  (bind _returnvalue (Game|GetPlayerController 0))
  ;[1 1 1] Clique do mouse na porta abre o inventario
  (Default|ToggleInventory (.AsFirst%20Person%20Character (Utilities|Casting|CastToFirstPersonCharacter (Game|Player|GetPlayerPawn 0))))
  ;[1 1 1] Ao entrar no trigger o mouse aparece
  (bind _output_get (Variables|/Script/Engine.PlayerController|SetbEnableClickEvents _returnvalue true))
  (Variables|/Script/Engine.PlayerController|SetbShowMouseCursor _returnvalue _output_get)
  (Input|SetInputModeGameandUI _returnvalue 0 false true))

(event OnComponentBeginOverlap(Trigger)
  (params (OverlappedComponent :type Primitive%20Component%20Object%20Reference) (OtherActor :type Actor%20Object%20Reference) (OtherComp :type Primitive%20Component%20Object%20Reference) (OtherBodyIndex :type Integer) (bFromSweep :type Boolean) (SweepResult :type Hit%20Result%20Structure%20%28by%20ref%29))
  (bind _returnvalue (Game|GetPlayerController 0))
  ;[1 1 1] Ao entrar no trigger o mouse aparece
  (if (not (Variables|Default|GetTrancada))
    ;[1 1 1] Evento para destrancar a porta
    (CallFunction|AbrePorta)
    (else
      (bind _output_get (Variables|/Script/Engine.PlayerController|SetbEnableClickEvents _returnvalue true))
      (Variables|/Script/Engine.PlayerController|SetbShowMouseCursor _returnvalue _output_get)
      (Input|SetInputModeGameandUI _returnvalue 0 false true))))

(event OnComponentEndOverlap(Trigger)
  (params (OverlappedComponent :type Primitive%20Component%20Object%20Reference) (OtherActor :type Actor%20Object%20Reference) (OtherComp :type Primitive%20Component%20Object%20Reference) (OtherBodyIndex :type Integer))
  (bind _returnvalue (Game|GetPlayerController 0))
  ;[1 1 1] Saida di trigger desabilita o mouse na tela
  (bind _output_get (Variables|/Script/Engine.PlayerController|SetbEnableClickEvents _returnvalue false))
  (Variables|/Script/Engine.PlayerController|SetbShowMouseCursor _returnvalue _output_get)
  (Input|SetInputModeGameOnly _returnvalue)
  (CallFunction|FechaPorta))

(event Custom|AbrePorta
  (bind _portaabrindo (Timeline|vai Play)
    (:Update
      (Transformation|SetRelativeRotation (Variables|Default|GetPorta) (Math|Rotator|MakeRotator 0.0 0.0 _portaabrindo) false false))))

(event Custom|Destranca
  ;[1 1 1] Evento para destrancar a porta
  (Variables|Default|SetTrancada false)
  (Default|HideInventory (.AsFirst%20Person%20Character (Utilities|Casting|CastToFirstPersonCharacter (Game|Player|GetPlayerPawn 0))))
  (CallFunction|AbrePorta))

(event Custom|FechaPorta
  (Utilities|FlowControl|Delay 0.5)
  (bind _portaabrindo (Timeline|vai Reverse)
    (:Update
      (Transformation|SetRelativeRotation (Variables|Default|GetPorta) (Math|Rotator|MakeRotator 0.0 0.0 _portaabrindo) false false))))

(event EventBeginPlay)

(event Collision|EventActorBeginOverlap
  (params (OtherActor :type Actor%20Object%20Reference)))

(event EventTick
  (params (DeltaSeconds :type Float%20%28single-precision%29)))

(fn ConstructionScript)